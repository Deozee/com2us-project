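; BP_InspectItem is an item inspection actor that displays a given mesh with a name and description widget.
; Inspect moves input from the character to itself; Interact returns it, removes the widget and destroys the actor.
; Mouse drag or move input rotates the mesh, the wheel zooms via clamped scene-capture FOV, and right-click resets both.
; External callers can set the item's initial rotation and scale.
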(event `/Game/Lee/BP/InteractInterface.Inspect`
  (params (Character :type "/Game/ThirdPerson/Blueprints/BP_FirstPersonCharacter Object Reference") (InsperctItem :type "StaticMesh Object Reference") (`Item Name` :type Text) (`Item Desc` :type Text))
  (bind _returnvalue (`GameplayStatics.GetPlayerController` 0))
  (set `self.Character` Character)
  (`StaticMeshComponent.SetStaticMesh` (`self.Item`) InsperctItem)
  (`SceneCaptureComponent.ShowOnlyActorComponents` (`self.SceneCaptureComponent2D`) (`self.Character`) true)
  (bind _returnvalue_2 (`|CreateWidget` "/Game/Lee/UI/W_Inspect.W_Inspect_C" null `Item Name` `Item Desc`))
  (bind _output_get (set `self.InspectWidgetRef` _returnvalue_2))
  (`UserWidget.AddToViewport` _output_get 0)
  (`self.DisableInput` (`self.Character`) _returnvalue)
  (`self.EnableInput` _returnvalue))

(event `EnhancedInput|/Game/ThirdPerson/Input/Actions/IA_Interact`
  (params (ActionValue :type Boolean) (ElapsedSeconds :type "Float (double-precision)") (TriggeredSeconds :type "Float (double-precision)") (InputAction :type "InputAction Object Reference" :default "/Game/ThirdPerson/Input/Actions/IA_Interact.IA_Interact"))
  (bind _returnvalue (`GameplayStatics.GetPlayerController` 0))
  (bind _inspectwidgetref (`self.InspectWidgetRef`))
  (:`Started`
    (`self.DisableInput` _returnvalue)
    (`self.EnableInput` (`self.Character`) _returnvalue)
    (`/Engine/EditorBlueprintResources/StandardMacros.IsValid` _inspectwidgetref
      (:`Is Valid`
        (`Widget.RemoveFromParent` _inspectwidgetref)
        (set `self.InspectWidgetRef` null)
        (`self.K2_DestroyActor`)))))

(event `set Inspect Rotation`
  (params (`Item Rotation` :type "Rotator Structure"))
  (bind _item (`self.Item`))
  (bind (_returnvalue_location _returnvalue_rotation _returnvalue_scale) (`KismetMathLibrary.BreakTransform` (`SceneComponent.K2_GetComponentToWorld` _item)))
  (bind _output_get (set `self.Item Rotation` `Item Rotation`))
  (`SceneComponent.K2_SetWorldTransform` _item (`KismetMathLibrary.MakeTransform` _returnvalue_location _output_get _returnvalue_scale) false false))

(event `Set Inspect Scale`
  (params (InspectionScale :type "Vector Structure"))
  (bind _item (`self.Item`))
  (bind (_returnvalue_location _returnvalue_rotation) (`KismetMathLibrary.BreakTransform` (`SceneComponent.K2_GetComponentToWorld` _item)))
  (`SceneComponent.K2_SetWorldTransform` _item (`KismetMathLibrary.MakeTransform` _returnvalue_location _returnvalue_rotation InspectionScale) false false))

(event `Key|LeftMouseButton`
  (params (Key :type "Key Structure"))
  ;[1 1 1] rotate item
  (:`Pressed`
    (set `self.Rotate?` true))
  (:`Released`
    (set `self.Rotate?` false)))

(event `Key|RightMouseButton`
  (params (Key :type "Key Structure"))
  ;[1 1 1] reset transform
  (:`Pressed`
    (`SceneComponent.K2_SetWorldRotation` (`self.Item`) (`self.Item Rotation`) false false)
    (set `SceneCaptureComponent2D.FOVAngle` 50.0 (`self.SceneCaptureComponent2D`))))

(event `Key|MouseScrollUp`
  (params (Key :type "Key Structure"))
  (bind _scenecapturecomponent2d (`self.SceneCaptureComponent2D`))
  ;[1 1 1] zoom In
  (:`Pressed`
    (set `SceneCaptureComponent2D.FOVAngle` (`KismetMathLibrary.FClamp` (- (`SceneCaptureComponent2D.FOVAngle` _scenecapturecomponent2d) 1.0) 30.0 80.0) _scenecapturecomponent2d)))

(event `InputAxisKey|MouseX`
  (params (AxisValue :type "Float (single-precision)"))
  ;[1 1 1] set Mousement horizontally
  (if (`self.Rotate?`)
    (`SceneComponent.K2_SetWorldRotation` (`self.Item`) (`KismetMathLibrary.ComposeRotators` (`SceneComponent.K2_GetComponentRotation` (`self.Item`)) (`KismetMathLibrary.MakeRotator` 0.0 0.0 (* AxisValue -3.0))) false false)))

(event `Key|MouseScrollDown`
  (params (Key :type "Key Structure"))
  (bind _scenecapturecomponent2d (`self.SceneCaptureComponent2D`))
  ;[1 1 1] zoom Out
  (:`Pressed`
    (set `SceneCaptureComponent2D.FOVAngle` (`KismetMathLibrary.FClamp` (+ (`SceneCaptureComponent2D.FOVAngle` _scenecapturecomponent2d) 1.0) 30.0 80.0) _scenecapturecomponent2d)))

(event `InputAxisKey|MouseY`
  (params (AxisValue :type "Float (single-precision)"))
  ;[1 1 1] set mouse vtically
  (if (`self.Rotate?`)
    (`SceneComponent.K2_SetWorldRotation` (`self.Item`) (`KismetMathLibrary.ComposeRotators` (`SceneComponent.K2_GetComponentRotation` (`self.Item`)) (`KismetMathLibrary.MakeRotator` 0.0 (* AxisValue -3.0))) false false)))

(event `EnhancedInput|/Game/ThirdPerson/Input/Actions/IA_Move`
  (params (ActionValue :type "Vector2D Structure") (ElapsedSeconds :type "Float (double-precision)") (TriggeredSeconds :type "Float (double-precision)") (InputAction :type "InputAction Object Reference" :default "/Game/ThirdPerson/Input/Actions/IA_Move.IA_Move"))
  ;[1 1 1] move with wasd
  (:`Triggered`
    (if (or (!= ActionValue_X 0.0) (!= ActionValue_Y 0.0))
      (`|ExecutionSequence`
        (:`then_0`
          (`SceneComponent.K2_SetWorldRotation` (`self.Item`) (`KismetMathLibrary.ComposeRotators` (`SceneComponent.K2_GetComponentRotation` (`self.Item`)) (`KismetMathLibrary.MakeRotator` 0.0 0.0 (* ActionValue_X -2.0))) false false))
        (:`then_1`
          (`SceneComponent.K2_SetWorldRotation` (`self.Item`) (`KismetMathLibrary.ComposeRotators` (`SceneComponent.K2_GetComponentRotation` (`self.Item`)) (`KismetMathLibrary.MakeRotator` 0.0 (* ActionValue_Y -2.0))) false false))))))

(fn `Interact`
  (params (Interact :type "Character Object Reference"))
  (return))

(fn `UserConstructionScript`)