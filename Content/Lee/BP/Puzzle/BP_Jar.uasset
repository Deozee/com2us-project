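; BP_Jar is a puzzle jar that, when interacted with, takes input from the player pawn and blends the camera to itself.
; WASD starts a timed world-axis move, which Tick applies unswept with offsets growing with elapsed time.
; Press flags gate repeated moves, but A and D only change the W/S flags, so PressA and PressD are never set.
; Only W uses the SetDirection helper, which prints its flag.
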(event `/Game/Lee/BP/Inspect/InteractInterface.Interacted`
  (params (Character :type "/Game/ThirdPerson/Blueprints/BP_FirstPersonCharacter Object Reference"))
  (bind _returnvalue (`GameplayStatics.GetPlayerController` 0))
  (`self.DisableInput` (`GameplayStatics.GetPlayerPawn` 0) _returnvalue)
  (`self.EnableInput` _returnvalue)
  (`PlayerController.SetViewTargetWithBlend` (`GameplayStatics.GetPlayerController` 0) self 1.0 "VTBlend_Linear" 0.0 false))

(event `self.ReceiveTick`
  (params (DeltaSeconds :type "Float (single-precision)"))
  (if (`self.IsMoving `)
    (bind _output_get (set `self.ElapsedTime ` (+ DeltaSeconds (`self.ElapsedTime `))))
    (if (< _output_get (`self.MoveDuration `))
      (`self.K2_AddActorWorldOffset` (* (`self.MoveDirection`) (`self.ElapsedTime `)))
      (else
        (set `self.IsMoving ` false)))))

(event `Key|W`
  (params (Key :type "Key Structure"))
  (bind _press_w (`self.Press W`))
  ;[1 1 1] 나중에 함 enum 으로 바꾸기
  (:`Pressed`
    (`self.Set Direction` (1.0 0.0 0.0) _press_w)
    (if _press_w
      (set `self.Press W` false)
      (set `self.Press S` false)
      (else
        (set `self.Press W` true)))))

(event `Key|S`
  (params (Key :type "Key Structure"))
  (:`Pressed`
    (if (`self.IsMoving `)
      _
      (elif (not (`self.Press S`))
        (set `self.MoveDirection` (-1.0 0.0 0.0))
        (set `self.IsMoving ` true)
        (set `self.ElapsedTime ` 0.0)
        (if (`self.Press W`)
          (set `self.Press S` false)
          (set `self.Press W` false)
          (else
            (set `self.Press S` true)))))))

(event `Key|A`
  (params (Key :type "Key Structure"))
  (:`Pressed`
    (if (`self.IsMoving `)
      _
      (elif (not (`self.Press A`))
        (set `self.MoveDirection` (0.0 -1.0 0.0))
        (set `self.IsMoving ` true)
        (set `self.ElapsedTime ` 0.0)
        (if (`self.Press S`)
          (set `self.Press W` false)
          (set `self.Press S` false)
          (else
            (set `self.Press W` true)))))))

(event `Key|D`
  (params (Key :type "Key Structure"))
  (:`Pressed`
    (if (`self.IsMoving `)
      _
      (elif (not (`self.Press D`))
        (set `self.MoveDirection` (0.0 1.0 0.0))
        (set `self.IsMoving ` true)
        (set `self.ElapsedTime ` 0.0)
        (if (`self.Press S`)
          (set `self.Press W` false)
          (set `self.Press S` false)
          (else
            (set `self.Press W` true)))))))

(fn `Set Direction`
  (params (vec :type "Vector Structure") (PressKey :type Boolean))
  (if (not (`self.IsMoving `))
    (`KismetSystemLibrary.PrintString` (`KismetStringLibrary.Conv_BoolToString` PressKey))
    (if (not PressKey)
      (set `self.MoveDirection` vec)
      (set `self.IsMoving ` true)
      (set `self.ElapsedTime ` 0.0))))

(fn `UserConstructionScript`)