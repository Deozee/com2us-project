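; BP_Item is an item actor that shows proximity icons based on how close the player character is.
; Two overlap spheres drive two icons: entering the outer sphere shows OutIcon, and entering the inner sphere swaps it for InnerIcon.
; Leaving each sphere reverses that change, and only the first player's character triggers it.
; The construction script sets both sphere radii from the InnerSphereRadius and OutSphereRadius variables.
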(event `self.InnerSphere.OnComponentBeginOverlap`
  (params (OverlappedComponent :type "PrimitiveComponent Object Reference") (OtherActor :type "Actor Object Reference") (OtherComp :type "PrimitiveComponent Object Reference") (OtherBodyIndex :type Integer) (bFromSweep :type Boolean) (SweepResult :type "HitResult Structure (by ref)"))
  (if (== OtherActor (`GameplayStatics.GetPlayerCharacter` 0))
    (`SceneComponent.SetVisibility` (`self.InnerIcon`) true false)
    (`SceneComponent.SetVisibility` (`self.OutIcon`) false false)))

(event `self.InnerSphere.OnComponentEndOverlap`
  (params (OverlappedComponent :type "PrimitiveComponent Object Reference") (OtherActor :type "Actor Object Reference") (OtherComp :type "PrimitiveComponent Object Reference") (OtherBodyIndex :type Integer))
  (if (== (`GameplayStatics.GetPlayerCharacter` 0) OtherActor)
    (`SceneComponent.SetVisibility` (`self.InnerIcon`) false false)
    (`SceneComponent.SetVisibility` (`self.OutIcon`) true false)))

(event `self.OuterSphere.OnComponentBeginOverlap`
  (params (OverlappedComponent :type "PrimitiveComponent Object Reference") (OtherActor :type "Actor Object Reference") (OtherComp :type "PrimitiveComponent Object Reference") (OtherBodyIndex :type Integer) (bFromSweep :type Boolean) (SweepResult :type "HitResult Structure (by ref)"))
  (if (== OtherActor (`GameplayStatics.GetPlayerCharacter` 0))
    (`SceneComponent.SetVisibility` (`self.OutIcon`) true false)))

(event `self.OuterSphere.OnComponentEndOverlap`
  (params (OverlappedComponent :type "PrimitiveComponent Object Reference") (OtherActor :type "Actor Object Reference") (OtherComp :type "PrimitiveComponent Object Reference") (OtherBodyIndex :type Integer))
  (if (== OtherActor (`GameplayStatics.GetPlayerCharacter` 0))
    (`SceneComponent.SetVisibility` (`self.OutIcon`) false false)))

(fn `UserConstructionScript`
  (`SphereComponent.SetSphereRadius` (`self.InnerSphere`) (`self.InnerSphere Radius`) true)
  (`SphereComponent.SetSphereRadius` (`self.OuterSphere`) (`self.OutSphere Radius`) true))